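; BP_albums is a VR prop that the motion controller can pick up and drop, playing a dialogue line when picked up.
; Pickup turns off physics and attaches the root to the grabbing component, while Drop re-enables physics and detaches it.
; It finds the SoundManager at BeginPlay and requests its dialogue on pickup until HasItBeenPlayed, set from that call's result, is true.
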(event `self.ReceiveBeginPlay`
  (bind _outactors (`GameplayStatics.GetAllActorsOfClass` "/Game/VirtualRealityBP/Blueprints/SoundManager.SoundManager_C"))
  (set `self.Smanager` (`|GetArrayItem` _outactors)))

(event `/Game/VirtualRealityBP/Blueprints/PickupActorInterface.Pickup`
  (params (AttachTo :type "SceneComponent Object Reference"))
  (`PrimitiveComponent.SetSimulatePhysics` (`self.StaticMeshComponent`) false)
  (`SceneComponent.K2_AttachToComponent` (`self.K2_GetRootComponent`) AttachTo "None" "KeepWorld" "KeepWorld" "KeepWorld" false)
  (if (not (`self.HasItBeenPlayed?`))
    (bind _hasitbeenplayed (`/Game/VirtualRealityBP/Blueprints/SoundManager.PlayDialogue` (`self.SManager`) 13))
    (set `self.HasItBeenPlayed?` _hasitbeenplayed)))

(event `/Game/VirtualRealityBP/Blueprints/PickupActorInterface.Drop`
  (`PrimitiveComponent.SetSimulatePhysics` (`self.StaticMeshComponent`) true)
  (`self.K2_DetachFromActor` "KeepWorld" "KeepWorld" "KeepWorld"))

(fn `UserConstructionScript`)