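; Toy car actor that can be picked up and dropped by BP_MotionController, triggering a line of dialogue when picked up.
; Pickup disables physics on CarBody and attaches the actor to the given component; Drop re-enables physics and detaches it.
; It finds the SoundManager at BeginPlay and requests the dialogue on pickup until HasItBeenPlayed, set from PlayDialogue's return value, becomes true.
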(event `self.ReceiveBeginPlay`
  (bind _outactors (`GameplayStatics.GetAllActorsOfClass` "/Game/VirtualRealityBP/Blueprints/SoundManager.SoundManager_C"))
  (set `self.SManager` (`|GetArrayItem` _outactors)))

(event `/Game/VirtualRealityBP/Blueprints/PickupActorInterface.Pickup`
  (params (AttachTo :type "SceneComponent Object Reference"))
  (`PrimitiveComponent.SetSimulatePhysics` (`self.car_body`) false)
  (`SceneComponent.K2_AttachToComponent` (`self.K2_GetRootComponent`) AttachTo "None" "KeepWorld" "KeepWorld" "KeepWorld" false)
  (if (not (`self.Has it been played?`))
    (bind _hasitbeenplayed (`/Game/VirtualRealityBP/Blueprints/SoundManager.PlayDialogue` (`self.SManager`) 0))
    (set `self.Has it been played?` _hasitbeenplayed)))

(event `/Game/VirtualRealityBP/Blueprints/PickupActorInterface.Drop`
  (`PrimitiveComponent.SetSimulatePhysics` (`self.car_body`) true)
  (`self.K2_DetachFromActor` "KeepWorld" "KeepWorld" "KeepWorld"))

(fn `UserConstructionScript`)